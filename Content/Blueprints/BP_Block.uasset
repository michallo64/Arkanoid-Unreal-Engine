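; BP_Block is a breakable block actor that awards points when a BP_Ball hits it.
; On a component hit from the ball it destroys itself, then passes its truncated Points value to BOGameMode's UpdateScore.
; Its construction script creates a dynamic instance of M_Basic and sets the Colour parameter from BlockColour, so each block carries its own colour.
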(event `self.Block.OnComponentHit`
  (params (HitComponent :type "PrimitiveComponent Object Reference") (OtherActor :type "Actor Object Reference") (OtherComp :type "PrimitiveComponent Object Reference") (NormalImpulse :type "Vector Structure") (Hit :type "HitResult Structure (by ref)"))
  (cast `/Game/Blueprints/BP_Ball` OtherActor)
  (`self.K2_DestroyActor`)
  (bind _asbogame_mode (cast `/Game/Blueprints/BOGameMode` (`GameplayStatics.GetGameMode`)))
  (`/Game/Blueprints/BOGameMode.Update Score` _asbogame_mode (`KismetMathLibrary.FTrunc` (`self.Points`))))

(fn `UserConstructionScript`
  (bind _returnvalue (`PrimitiveComponent.CreateDynamicMaterialInstance` (`self.Block`) 0 "/Game/Materials/M_Basic.M_Basic" "None"))
  (`MaterialInstanceDynamic.SetVectorParameterValue` _returnvalue "Colour" (`self.BlockColour`)))